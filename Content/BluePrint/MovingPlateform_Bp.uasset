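; Moving platform actor that shuttles its static mesh back and forth between two points indefinitely.
; On BeginPlay it stores the actor's location as the start and treats EndPosition as an offset from it.
; A looping MoveComponentTo feeds these world-derived points in as relative targets, swapping target after each move.
; MovSpeed sets the duration of each leg, not a velocity.
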(event EventBeginPlay
  (bind _returnvalue (Transformation|GetActorLocation))
  (Variables|Default|SetStartPosition _returnvalue)
  (bind _output_get (Variables|Default|SetEndPosition (+ _returnvalue (Variables|Default|GetEndPosition))))
  (Variables|Default|SetTargetPosition _output_get)
  (Components|MoveComponentTo (Variables|Default|GetStaticMesh) (Variables|Default|GetTargetPosition) "0, 0, 0" false false (Variables|Default|GetMovSpeed) false :!label _label)
  (if (Math|Vector|Equal(Vector) (Variables|Default|GetStartPosition) (Variables|Default|GetTargetPosition) 0.0001)
    (Variables|Default|SetTargetPosition (Variables|Default|GetEndPosition))
    (goto _label)
    (else
      (Variables|Default|SetTargetPosition (Variables|Default|GetStartPosition))
      (goto _label))))

(fn ConstructionScript)