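; Player Blueprint for movement, jumping, score and the game-over state.
; Axis inputs drive movement input along actor forward and right vectors, and jump applies an upward impulse to the StaticMesh when grounded.
; Upward-normal hits set Grounded, while the left/right axis event clears it during play.
; ADDSCORE accumulates score; GAMEOverFunction shows the end-screen widget and cursor, setting a flag that blocks input.
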(event OnComponentBeginOverlap(StaticMesh)
  (params (OverlappedComponent :type Primitive%20Component%20Object%20Reference) (OtherActor :type Actor%20Object%20Reference) (OtherComp :type Primitive%20Component%20Object%20Reference) (OtherBodyIndex :type Integer) (bFromSweep :type Boolean) (SweepResult :type Hit%20Result%20Structure%20%28by%20ref%29)))

(event Collision|EventHit
  (params (MyComp :type Primitive%20Component%20Object%20Reference) (Other :type Actor%20Object%20Reference) (OtherComp :type Primitive%20Component%20Object%20Reference) (bSelfMoved :type Boolean) (HitLocation :type Vector :default "0, 0, 0") (HitNormal :type Vector :default "0, 0, 0") (NormalImpulse :type Vector :default "0, 0, 0") (Hit :type Hit%20Result%20Structure%20%28by%20ref%29))
  (if (Math|Vector|Equal(Vector) HitNormal "0, 0,1.000000" 0.0001)
    (Variables|Default|SetGrounded true)))

(event EventBeginPlay)

(event Input|ActionEvents|InputActionJUMPSKEY
  (params (Key :type Key%20Structure :default "None"))
  (:Pressed
    (if (Variables|Default|GetGrounded)
      (if (not (Variables|Default|GetisGameClearOrGameOver))
        (Physics|AddImpulse (Variables|Default|GetStaticMesh) (* (Math|Vector|VectorUp) (Variables|Default|GetJUMPForce)) "None" true)))))

(event Input|AxisEvents|InputAxisMOVFORWARDBack
  (params (AxisValue :type Float%20%28single-precision%29))
  (if (not (Variables|Default|GetisGameClearOrGameOver))
    (Pawn|Input|AddMovementInput (Math|Vector|GetForwardVector (Transformation|GetActorRotation)) AxisValue false)))

(event Input|AxisEvents|InputAxisMOVLEFTRIGHT
  (params (AxisValue :type Float%20%28single-precision%29))
  (if (not (Variables|Default|GetisGameClearOrGameOver))
    (Pawn|Input|AddMovementInput (Math|Vector|GetRightVector (Transformation|GetActorRotation)) AxisValue false)
    (Variables|Default|SetGrounded false)))

(fn ConstructionScript)

(fn ADDSCORE
  (params (SCOREValEarn :type Integer))
  (Variables|Default|SetSCORE (+ (Variables|Default|GetSCORE) SCOREValEarn)))

(fn GAMEOverFunction
  (if (not (Variables|Default|GetisGameClearOrGameOver))
    (bind _returnvalue (UserInterface|CreateWidget "/Game/BluePrint/ENDGameUI_BP.ENDGameUI_BP_C"))
    (UserInterface|Viewport|AddtoViewport _returnvalue 0)
    (Default|SETEndScreenFunction _returnvalue false)
    (Variables|Default|SetisGameClearOrGameOver true)
    (Variables|/Script/Engine.PlayerController|SetbShowMouseCursor (Game|GetPlayerController 0) true)))