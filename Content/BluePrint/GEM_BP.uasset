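; GEM_BP is a collectible gem that awards score when the player touches it.
; On overlap with a Player_BP, it passes ScoreTOGiven to that player's ADDSCORE and destroys itself.
; Each tick it yaws the mesh by RotateSpd scaled by delta time, also adding the actor's roll and pitch.
; A sine of real time is added to the mesh's height each frame, producing a frame-rate-dependent bob.
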(event Collision|EventActorBeginOverlap
  (params (OtherActor :type Actor%20Object%20Reference))
  (bind _asplayer_bp (Utilities|Casting|CastToPlayer_BP OtherActor))
  (Default|ADDSCORE _asplayer_bp (Variables|Default|GetScoreTOGiven))
  (Actor|DestroyActor))

(event EventTick
  (params (DeltaSeconds :type Float%20%28single-precision%29))
  (bind _returnvalue (Transformation|GetActorRotation))
  (bind (_roll _pitch) (Math|Rotator|BreakRotator _returnvalue))
  (Transformation|AddWorldRotation (Variables|Default|GetStaticMesh_GEM) (Math|Rotator|MakeRotator _roll _pitch (* DeltaSeconds (Variables|Default|GetRotateSpd))) false false)
  (Transformation|AddWorldOffset (Variables|Default|GetStaticMesh_GEM) (Math|Vector|MakeVector 0.0 0.0 (Math|Trig|Sin(Radians) (Utilities|Time|GetRealTimeSeconds))) false false))

(fn ConstructionScript)