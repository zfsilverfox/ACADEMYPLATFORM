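; Enemy Blueprint that patrols back and forth between two points and triggers game over when the player overlaps it.
; On BeginPlay it stores the actor location as the start and adds the ENDPosition offset to form the end.
; A looping MoveComponentTo moves the StaticMesh's relative location over MovSpd seconds, flipping the target on completion.
; Actor overlap casts to Player_BP and calls its GAMEOverFunction.
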(event EventBeginPlay
  (bind _returnvalue (Transformation|GetActorLocation))
  (Variables|Default|SetStartPosition _returnvalue)
  (Variables|Default|SetENDPosition (+ _returnvalue (Variables|Default|GetENDPosition)))
  (Variables|Default|SetTargetPosition (Variables|Default|GetENDPosition))
  (Components|MoveComponentTo (Variables|Default|GetStaticMesh) (Variables|Default|GetTargetPosition) "0, 0, 0" false false (Variables|Default|GetMovSpd) false :!label _label)
  (if (Math|Vector|Equal(Vector) (Variables|Default|GetTargetPosition) (Variables|Default|GetStartPosition) 0.0001)
    (Variables|Default|SetTargetPosition (Variables|Default|GetENDPosition))
    (goto _label)
    (else
      (Variables|Default|SetTargetPosition (Variables|Default|GetStartPosition))
      (goto _label))))

(event Collision|EventActorBeginOverlap
  (params (OtherActor :type Actor%20Object%20Reference))
  (bind _asplayer_bp (Utilities|Casting|CastToPlayer_BP OtherActor))
  (Default|GAMEOverFunction _asplayer_bp))

(fn ConstructionScript)